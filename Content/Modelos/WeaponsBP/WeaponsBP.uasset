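; WeaponsBP is a pickup weapon actor that the player equips into the character's right-hand socket.
; Overlapping its Collision component enables player input, and ending overlap on the Weapon component disables it.
; The Equip action calls EQUIP, which snaps the Weapon component to RHsocket on the player character's mesh.
; A trailing cast of that mesh to ThirdPersonCharacter drives no further logic.
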(event OnComponentBeginOverlap(Collision)
  (params (OverlappedComponent :type Primitive%20Component%20Object%20Reference) (OtherActor :type Actor%20Object%20Reference) (OtherComp :type Primitive%20Component%20Object%20Reference) (OtherBodyIndex :type Integer) (bFromSweep :type Boolean) (SweepResult :type Hit%20Result%20Structure%20%28by%20ref%29))
  (Input|EnableInput (Game|GetPlayerController 0)))

(event OnComponentEndOverlap(weapon)
  (params (OverlappedComponent :type Primitive%20Component%20Object%20Reference) (OtherActor :type Actor%20Object%20Reference) (OtherComp :type Primitive%20Component%20Object%20Reference) (OtherBodyIndex :type Integer))
  (Input|DisableInput (Game|GetPlayerController 0)))

(event EventBeginPlay)

(event Collision|EventActorBeginOverlap
  (params (OtherActor :type Actor%20Object%20Reference)))

(event EventTick
  (params (DeltaSeconds :type Float%20%28single-precision%29)))

(event Input|ActionEvents|InputActionEquip
  (params (Key :type Key%20Structure :default "None"))
  (:Pressed
    (CallFunction|EQUIP)))

(fn ConstructionScript)

(fn EQUIP
  (bind _returnvalue (Game|GetPlayerCharacter 0))
  (bind _mesh (Variables|/Script/Engine.Character|GetMesh _returnvalue))
  (Transformation|AttachComponentToComponent (Variables|Default|Getweapon) _mesh "RHsocket" "SnapToTarget" "SnapToTarget" "SnapToTarget" true)
  (Utilities|Casting|CastToThirdPersonCharacter _mesh))